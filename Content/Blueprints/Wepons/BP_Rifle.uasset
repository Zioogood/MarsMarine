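; Rifle weapon Blueprint that handles automatic hitscan fire through SVR_ fire and stop events.
; Firing checks player 0's ammo once, then activates a particle effect and repeats a line trace on a looping timer; without ammo it plays an empty sound.
; Each trace runs forward from the muzzle socket, applying damage and spawning an impact emitter on blocking hits.
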(event `SVR_WeponFire`
  (`self.StartFire`))

(event `SVR_StopFire`
  (`self.StopFire`))

(fn `NoAmmo`
  (`ActorComponent.Deactivate` (`self.ParticleSystem`))
  (`KismetSystemLibrary.K2_ClearTimer` null "Weapon Trace")
  (bind _returnvalue (`GameplayStatics.SpawnSound2D` "/Game/Sounds/Weapon_AssaultRifle/Stereo/EmptyRiffleSound.EmptyRiffleSound" 1.0 1.0 0.0 null))
  (set `self.SoundEffect` _returnvalue)
  (return))

(fn `Spawn Impact Hit`
  (params (`Hit Location` :type "Vector Structure"))
  (`GameplayStatics.SpawnEmitterAtLocation` "/Game/Effects/Weapons/Impacts/P_AssaultRifle_IH.P_AssaultRifle_IH" `Hit Location`))

(fn `StartFire`
  (bind _asbp_player_character (cast `/Game/Blueprints/Pawns/BP_PlayerCharacter` (`GameplayStatics.GetPlayerCharacter` 0)))
  (if (`/Game/Blueprints/Pawns/BP_PlayerCharacter.HaveAmmo` _asbp_player_character)
    (`ActorComponent.Activate` (`self.ParticleSystem`) false)
    (`self.Weapon Trace`)
    (`KismetSystemLibrary.K2_SetTimer` null "Weapon Trace" (`self.Time`) true)
    (else
      (`self.NoAmmo`))))

(fn `StopFire`
  (`ActorComponent.Deactivate` (`self.ParticleSystem`))
  (`KismetSystemLibrary.K2_ClearTimer` null "Weapon Trace")
  (return))

(fn `TranceEndLocation`
  (returns (ReturnValue :type "Vector Structure"))
  (return (+ (`self.TranceStartLocation`) (* (`KismetMathLibrary.Conv_RotatorToVector` (`SceneComponent.GetSocketRotation` (`self.Rifle1`) "MuzzleFlashSocket")) (`self.WeaponRange`)))))

(fn `TranceStartLocation`
  (returns (ReturnValue :type "Vector Structure"))
  (return (`SceneComponent.GetSocketLocation` (`self.Rifle1`) "MuzzleFlashSocket")))

(fn `UserConstructionScript`)

(fn `Weapon Trace`
  (bind _outhit (`KismetSystemLibrary.LineTraceSingle` (`self.TranceStartLocation`) (`self.TranceEndLocation`) "TraceTypeQuery1" false (`|MakeArray` (`GameplayStatics.GetPlayerCharacter` 0) :!type "Actor Object Reference")))
  (bind (_bblockinghit _binitialoverlap _time _distance _location _impactpoint _normal _impactnormal _physmat _hitactor) (`GameplayStatics.BreakHitResult` _outhit))
  (if _bblockinghit
    (`GameplayStatics.ApplyDamage` _hitactor (`self.WeaponDamage`))
    (`self.Spawn Impact Hit` _location)))