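; Level exit trigger that completes the level when the player overlaps it with enough kills and no aliens left.
; The kill target scales with the level's position in the LevelName array, and the alien check reads the Alien array on BP_MarsMarineGameMode.
; On completion it opens the next level in that array, or prints a win message and quits on the final level.
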(event `self.ReceiveActorBeginOverlap`
  (params (OtherActor :type "Actor Object Reference"))
  (`/Game/Blueprints/Librery/CC_MacroLibrerys.Is Player` OtherActor
    (:`Player`
      (if (and (`self.KillsCalculator`) (`self.Is Alien in World`))
        (`self.Complete Level`)))))

(fn `Complete Level`
  (if (`self.Is Finale Level`)
    (`KismetSystemLibrary.PrintString` "you win game ")
    (`KismetSystemLibrary.QuitGame` null "Quit")
    (else
      (`self.Load Next Level`))))

(fn `Get Current Level Index`
  (returns (LevelName :type Integer))
  (bind _returnvalue (`GameplayStatics.GetCurrentLevelName` true))
  (return (`KismetArrayLibrary.Array_Find` (`self.Level Name`) (`KismetStringLibrary.Conv_StringToName` _returnvalue))))

(fn `Get Next Level`
  (returns (Output :type Name))
  (return (`|GetArrayItem` (`self.Level Name`) (+ (`self.Get Current Level Index`) 1))))

(fn `Is Alien in World`
  (returns (ReturnValue :type Boolean))
  (bind _returnvalue (`GameplayStatics.GetActorOfClass` "/Game/Blueprints/GameMode/BP_MarsMarineGameMode.BP_MarsMarineGameMode_C"))
  (return (== (`KismetArrayLibrary.Array_Length` (`/Game/Blueprints/GameMode/BP_MarsMarineGameMode.Alien` _returnvalue)) 0)))

(fn `Is Finale Level`
  (returns (ReturnValue :type Boolean))
  (return (== (`KismetArrayLibrary.Array_LastIndex` (`self.Level Name`)) (`self.Get Current Level Index`))))

(fn `KillsCalculator`
  (returns (ReturnValue :type Boolean))
  (bind _asbp_player_character (cast `/Game/Blueprints/Pawns/BP_PlayerCharacter` (`GameplayStatics.GetPlayerPawn` 0)))
  (return (>= (`/Game/Blueprints/Pawns/BP_PlayerCharacter.Kills` _asbp_player_character) (`self.LevelDifficulty`))))

(fn `LevelDifficulty`
  (returns (Output_Get :type Integer))
  (bind _output_get (set `self.Win Condytion` (* (+ (`self.Get Current Level Index`) 1) 40)))
  (return _output_get))

(fn `Load Next Level`
  (`GameplayStatics.OpenLevel` (`self.Get Next Level`)))

(fn `UserConstructionScript`)