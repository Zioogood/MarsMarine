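; BP_Start_Wave_Trigger is a trigger actor that signals the start of a wave when the player overlaps it.
; It checks BP_MarsMarineGameMode and fires only while no alien is in the world.
; The signal is a brief pulse: StartWave turns true, then resets after a short Delay.
; SetStartWave, despite its name, only returns the inverse of that flag; nothing here spawns enemies.
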(event `self.ReceiveActorBeginOverlap`
  (params (OtherActor :type "Actor Object Reference"))
  (`/Game/Blueprints/Librery/CC_MacroLibrerys.Is Player` OtherActor
    (:`Player`
      (bind _asbp_mars_marine_game_mode (cast `/Game/Blueprints/GameMode/BP_MarsMarineGameMode` (`GameplayStatics.GetGameMode`)))
      (if (not (`/Game/Blueprints/GameMode/BP_MarsMarineGameMode.IsAlienInWorld` _asbp_mars_marine_game_mode))
        (set `self.StartWave` true)
        (`KismetSystemLibrary.Delay` 0.2)
        (set `self.StartWave` false)))))

(fn `Set Start Wave`
  (returns (ReturnValue :type Boolean))
  (return (not (`self.StartWave`))))

(fn `UserConstructionScript`)