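; Game mode for a Mars marine shooter that plays music and runs waves of aliens spawned at random TargetPoints.
; Tick polls BP_Start_Wave_Trigger to start waves, while SetupNewWave checks BP_Lvl1_WinCondytion's kill calculator before scaling difficulty from level index and previous wave size.
; A looping timer spawns aliens until the quota runs out.
; Registered deaths empty the alien array, triggering the next wave after a delay.
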(event `self.ReceiveBeginPlay`
  (bind _returnvalue (`GameplayStatics.SpawnSound2D` "/Game/Sounds/Music/ShooterGame_Music_Cue.ShooterGame_Music_Cue" 1.0 1.0 0.0 null))
  (set `self.Sound Effect` _returnvalue))

(event `self.ReceiveTick`
  (params (DeltaSeconds :type "Float (single-precision)"))
  (bind _returnvalue (`GameplayStatics.GetActorOfClass` "/Game/Blueprints/Trigger/BP_Start_Wave_Trigger.BP_Start_Wave_Trigger_C"))
  (if (`/Game/Blueprints/Trigger/BP_Start_Wave_Trigger.StartWave` _returnvalue)
    (`KismetSystemLibrary.Delay` 0.2)
    (`self.Setup New Wave`)))

(event `Spawn Wave`
  (`self.SpawnAlien`))

(event `End Wave`
  (`KismetSystemLibrary.Delay` 2.0)
  (`self.Setup New Wave`))

(fn `Get RandomSpawn Point`
  (returns (SpawnPoint :type "TargetPoint Object Reference"))
  (bind _outactors (`GameplayStatics.GetAllActorsOfClass` "/Script/Engine.TargetPoint"))
  (return (`|GetArrayItem` _outactors (`KismetMathLibrary.RandomIntegerInRange` 0 (`KismetArrayLibrary.Array_LastIndex` _outactors)))))

(fn `Increase Wave Difficulty`
  (bind _returnvalue (`GameplayStatics.GetActorOfClass` "/Game/Blueprints/Trigger/BP_Lvl1_WinCondytion.BP_Lvl1_WinCondytion_C"))
  (bind _result (`/Engine/EditorBlueprintResources/StandardMacros.IncrementInt` (`/Game/Blueprints/Trigger/BP_Lvl1_WinCondytion.Get Current Level Index` _returnvalue))
    (:`  `
      (bind _output_get (set `self.Wave Dificulty` (+ (* _result 2) (`KismetMathLibrary.Round` (* (`self.Wave Dificulty`) (`self.Difficulty`))))))
      (set `self.Alien Spawn Remaning` _output_get))))

(fn `Is Wave Complete`
  (returns (ReturnValue :type Boolean))
  (return (and (== (`KismetArrayLibrary.Array_Length` (`self.Alien`)) 0) (== (`self.Alien Spawn Remaning`) 0))))

(fn `RegisterAlienDeath`
  (params (Alien :type "/Game/Blueprints/AI/BP_Alien Object Reference (by ref)"))
  (`KismetArrayLibrary.Array_RemoveItem` (`self.Alien`) Alien)
  (if (`self.Is Wave Complete`)
    (`self.End Wave`)))

(fn `Setup New Wave`
  (bind _returnvalue (`GameplayStatics.GetActorOfClass` "/Game/Blueprints/Trigger/BP_Lvl1_WinCondytion.BP_Lvl1_WinCondytion_C"))
  (if (not (`/Game/Blueprints/Trigger/BP_Lvl1_WinCondytion.KillsCalculator` _returnvalue))
    (`/Engine/EditorBlueprintResources/StandardMacros.IncrementInt` (`self.Current Wave`)
      (:`  `
        (`self.Increase Wave Difficulty`)
        (`KismetSystemLibrary.K2_SetTimer` null "Spawn Wave" 1.0 true)
        (return)))))

(fn `SpawnAlien`
  (set `self.IsAlienInWorld` true)
  (bind _spawnpoint (`self.Get RandomSpawn Point`))
  (`/Engine/EditorBlueprintResources/StandardMacros.IsValid` _spawnpoint
    (:`Is Valid`
      (bind _returnvalue (`|SpawnActorFromClass` "/Game/Blueprints/AI/BP_Alien.BP_Alien_C" (`self.GetTransform` _spawnpoint) "Undefined" "OverrideRootScale" null null))
      (`/Engine/EditorBlueprintResources/StandardMacros.IsValid` _returnvalue
        (:`Is Valid`
          (`KismetArrayLibrary.Array_Add` (`self.Alien`) _returnvalue)
          (bind _result (`/Engine/EditorBlueprintResources/StandardMacros.DecrementInt` (`self.Alien Spawn Remaning`))
            (:`  `
              (if (== _result 0)
                (`KismetSystemLibrary.K2_ClearTimer` null "Spawn Wave")
                (return)))))))))

(fn `UserConstructionScript`)